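; Player Blueprint for procedural swords, handling melee hit detection and test inputs.
; Blade and tip collision overlaps apply slash or stab damage from SwordAttributes, with knockback, through BPI_Damage.
; CanHit uses the HitActors list to block repeat hits on the same actor.
; Enhanced Input actions toggle the in-game generator widget with matching cursor and input mode, adjust its sword view, and spawn test enemies at a spawn point.
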(event OnComponentBeginOverlap(SwordCollisionComp)
  (params (OverlappedComponent :type Primitive%20Component%20Object%20Reference) (OtherActor :type Actor%20Object%20Reference) (OtherComp :type Primitive%20Component%20Object%20Reference) (OtherBodyIndex :type Integer) (bFromSweep :type Boolean) (SweepResult :type Hit%20Result%20Structure%20%28by%20ref%29))
  ;[0.15 0.15 0.15 0.5] slash collision
  (if (CallFunction|CanHit OtherActor)
    (Class|BPIDamage|ApplyDamage(Message) OtherActor (.SlashDamage (Utilities|Struct|BreakProcSwordAttributes (Variables|Default|GetSwordAttributes))) (Class|ProcPlayerCharacter|GetKnockback OtherActor 1e+02 2.5e+02))
    (Utilities|Set|Add (Variables|Default|GetHitActors) (Utilities|ResolveSoftReference OtherActor))))

(event OnComponentBeginOverlap(SwordTipCollisionComp)
  (params (OverlappedComponent :type Primitive%20Component%20Object%20Reference) (OtherActor :type Actor%20Object%20Reference) (OtherComp :type Primitive%20Component%20Object%20Reference) (OtherBodyIndex :type Integer) (bFromSweep :type Boolean) (SweepResult :type Hit%20Result%20Structure%20%28by%20ref%29))
  ;[0.15 0.15 0.15 0.5] stab collision
  (if (CallFunction|CanHit OtherActor)
    (Class|BPIDamage|ApplyDamage(Message) OtherActor (.StabDamage (Utilities|Struct|BreakProcSwordAttributes (Variables|Default|GetSwordAttributes))) (Class|ProcPlayerCharacter|GetKnockback OtherActor 1e+02 2.5e+02))
    (Utilities|Set|Add (Variables|Default|GetHitActors) (Utilities|ResolveSoftReference OtherActor))))

(event Input|EnhancedActionEvents|EnhancedInputActionIA_SpawnEnemy
  (params (ActionValue :type Boolean) (ElapsedSeconds :type Float%20%28double-precision%29) (TriggeredSeconds :type Float%20%28double-precision%29) (InputAction :type Input%20Action%20Object%20Reference :default "/Game/ProceduralSwords/Inputs/IA_SpawnEnemy.IA_SpawnEnemy"))
  ;[0.15 0.15 0.15 0.5] Spawn enemy
  (:Started
    (bind _returnvalue (Actor|GetActorOfClass "/Game/ProceduralSwords/BP_EnemySpawnPoint.BP_EnemySpawnPoint_C"))
    (Game|SpawnActorfromClass "/Game/ProceduralSwords/BP_TestEnemy.BP_TestEnemy_C" (Math|Transform|MakeTransform (Transformation|GetActorLocation _returnvalue)) "AlwaysSpawn" "MultiplyWithRoot" 0 0)))

(event Input|EnhancedActionEvents|EnhancedInputActionIA_SpawnGenerator
  (params (ActionValue :type Boolean) (ElapsedSeconds :type Float%20%28double-precision%29) (TriggeredSeconds :type Float%20%28double-precision%29) (InputAction :type Input%20Action%20Object%20Reference :default "/Game/ProceduralSwords/Inputs/Menu/IA_SpawnGenerator.IA_SpawnGenerator"))
  (bind _returnvalue (Game|GetPlayerController 0))
  (bind _returnvalue_2 (Game|GetPlayerController 0))
  ;[0.15 0.15 0.15 0.5] Spawn and despawn generator widget
  (:Started
    (Utilities|IsValid (Variables|Default|GetGeneratorWidget)
      (:Is%20Valid
        ;;[0.15 0.15 0.15 0.5] Remove widget
        (Widget|RemovefromParent (Variables|Default|GetGeneratorWidget))
        (Variables|Default|SetGeneratorWidget 0)
        ;;[0.15 0.15 0.15 0.5] Set cursor to game
        (Input|SetInputModeGameOnly _returnvalue_2 false)
        (Class|WidgetBlueprintLibrary|SetFocustoGameViewport)
        (Variables|/Script/Engine.PlayerController|SetbShowMouseCursor _returnvalue_2 false))
      (:Is%20Not%20Valid
        ;;[0.15 0.15 0.15 0.5] Spawn new
        (bind _returnvalue_3 (UserInterface|CreateWidget "/ProceduralSwordGenerator/UI/WBP_InGameGenerator.WBP_InGameGenerator_C" (Game|GetPlayerController 0)))
        (bind _output_get (Variables|Default|SetGeneratorWidget _returnvalue_3))
        (UserInterface|Viewport|AddtoViewport _output_get 0)
        ;;[0.15 0.15 0.15 0.5] Set cursor to widget
        (Input|SetInputModeGameandUI _returnvalue 0 "DoNotLock" false false)
        (Variables|/Script/Engine.PlayerController|SetbShowMouseCursor _returnvalue true)))))

(event Input|EnhancedActionEvents|EnhancedInputActionIA_SwapSwordView
  (params (ActionValue :type Boolean) (ElapsedSeconds :type Float%20%28double-precision%29) (TriggeredSeconds :type Float%20%28double-precision%29) (InputAction :type Input%20Action%20Object%20Reference :default "/Game/ProceduralSwords/Inputs/IA_SwapSwordView.IA_SwapSwordView"))
  (bind _generatorwidget (Variables|Default|GetGeneratorWidget))
  (:Started
    (Utilities|IsValid _generatorwidget
      (:Is%20Valid
        (Class|ProcinGameGeneratorWidget|AdjustSwordView _generatorwidget)))))

(event EventBeginPlay)

(event Collision|EventActorBeginOverlap
  (params (OtherActor :type Actor%20Object%20Reference)))

(event EventTick
  (params (DeltaSeconds :type Float%20%28single-precision%29)))

(fn ConstructionScript)

(fn CanHit
  (params (OtherActor :type Actor%20Object%20Reference))
  (if (not (Utilities|Set|Contains (Variables|Default|GetHitActors) (Utilities|ResolveSoftReference OtherActor)))
    (if (Utilities|DoesObjectImplementInterface OtherActor "/Game/ProceduralSwords/BPI_Damage.BPI_Damage_C")
      (return true)
      (else
        (return false)))
    (else
      (return false))))