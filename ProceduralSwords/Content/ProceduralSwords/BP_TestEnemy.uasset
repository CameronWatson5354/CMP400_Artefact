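; BP_TestEnemy is a test enemy character that walks toward BP_Player until it dies.
; ApplyDamage launches it with the given knockback in Falling mode, lowers health and spawns a floating damage-number widget actor.
; SetHealth refreshes the widget health bar, which assumes a fixed health range rather than a max-health variable.
; At zero health it stops chasing and destroys itself after DespawnTime.
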(event EventBeginPlay
  (Pawn|SpawnDefaultController)
  (bind _returnvalue (Actor|GetActorOfClass "/Game/ProceduralSwords/BP_Player.BP_Player_C"))
  (Variables|Default|SetPlayer _returnvalue)
  (bind _aswbp_enemy_health_bar (Utilities|Casting|CastToWBP_EnemyHealthBar (UserInterface|GetWidget (Variables|Default|GetWidget))))
  (Variables|Default|SetHealthBar _aswbp_enemy_health_bar)
  (CallFunction|UpdateHealthBar))

(event Collision|EventActorBeginOverlap
  (params (OtherActor :type Actor%20Object%20Reference)))

(event EventTick
  (params (DeltaSeconds :type Float%20%28single-precision%29))
  (if (not (Variables|Default|GetIsDead))
    (CallFunction|MoveTowardsPlayer)))

(event EventApplyDamage
  (params (Damage :type Float%20%28double-precision%29) (Knockback :type Vector :default "0, 0, 0"))
  (Variables|/Script/Engine.MovementComponent|SetVelocity (Variables|Character|GetCharacterMovement) Knockback)
  (Pawn|Components|CharacterMovement|SetMovementMode (Variables|Character|GetCharacterMovement) "MOVE_Falling" 0)
  (CallFunction|SetHealth (- (Variables|Default|GetHealth) Damage))
  (bind _returnvalue (Game|SpawnActorfromClass "/Game/ProceduralSwords/A_DamageNumber.A_DamageNumber_C" (Math|Transform|MakeTransform (+ (Transformation|GetActorLocation) "0.000000,50.000000,50.000000")) "Undefined" "MultiplyWithRoot" 0 0))
  (bind _aswbp_damage_number (Utilities|Casting|CastToWBP_DamageNumber (UserInterface|GetWidget (Variables|/Game/ProceduralSwords/A_DamageNumber.A_DamageNumber_C|GetWidget _returnvalue))))
  (Variables|/Script/UMG.TextBlock|SetText (Variables|/Game/ProceduralSwords/WBP_DamageNumber.WBP_DamageNumber_C|GetTXT_Damage _aswbp_damage_number) (Utilities|Text|ToText(Float) Damage "HalfToEven" false true 1 324 0 1)))

(fn ConstructionScript)

(fn SetHealth
  (params (NewHealth :type Float%20%28double-precision%29))
  (Variables|Default|SetHealth (Math|Float|Clamp(Float) NewHealth 0.0 999999.0))
  (CallFunction|UpdateHealthBar)
  ;[0.15 0.15 0.15 0.5] Checks and handles if the unit dies
  (if (<= (Variables|Default|GetHealth) 0.0)
    (Variables|Default|SetIsDead true)
    (Utilities|Time|SetTimerbyFunctionName 0 "DestroyEnemy" (Variables|Default|GetDespawnTime))))

(fn MoveTowardsPlayer
  (Class|PawnMovementComponent|AddInputVector (Variables|Character|GetCharacterMovement) (Class|KismetMathLibrary|VectorNormal2D (- (Transformation|GetActorLocation (Variables|Default|GetPlayer)) (Transformation|GetActorLocation)) 0.0001) false))

(fn DestroyEnemy
  (Actor|DestroyActor))

(fn UpdateHealthBar
  (Progress|SetPercent (Variables|/Game/ProceduralSwords/WBP_EnemyHealthBar.WBP_EnemyHealthBar_C|GetHealthBar (Variables|Default|GetHealthBar)) (Math|Float|NormalizetoRange (Variables|Default|GetHealth) 0.0 5e+01))
  (return))